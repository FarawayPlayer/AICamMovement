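; BP_Cam is a sensing actor, apparently a security camera, that alerts Guard_AI actors when it perceives the first-person player.
; AIPerception sightings wait one second, re-check the stimulus, then send every guard with a matching GroupID to investigate the player's location, passing along PatrolPoints.
; Debug prints and colored boxes mark detection and loss.
; PawnSensing is activated at BeginPlay, but its activation event only prints a message.
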(event `self.ReceiveBeginPlay`
  (`ActorComponent.Activate` (`self.PawnSensing`) false))

(event `self.PawnSensing.OnComponentActivated`
  (params (Component :type "ActorComponent Object Reference") (bReset :type Boolean))
  (`KismetSystemLibrary.PrintString` "Target Seen "))

(event `self.AIPerception.OnTargetPerceptionUpdated`
  (params (Actor :type "Actor Object Reference") (Stimulus :type "AIStimulus Structure"))
  (bind (_age _expirationage _strength _stimuluslocation _receiverlocation _tag _bsuccessfullysensed) (break `AIStimulus` Stimulus))
  (bind _asbp_first_person_character (cast `/Game/FirstPerson/Blueprints/BP_FirstPersonCharacter` Actor))
  (if _bsuccessfullysensed
    (`KismetSystemLibrary.PrintString` "Target Spotted")
    (`KismetSystemLibrary.Delay` 1.0)
    (if _bsuccessfullysensed
      (`KismetSystemLibrary.PrintString` "Still Seen")
      (bind _returnvalue (`SceneComponent.K2_GetComponentLocation` (`Character.CapsuleComponent` _asbp_first_person_character)))
      (`KismetSystemLibrary.DrawDebugBox` _returnvalue (0.0 0.0 0.0) (struct :`G` 1.0 :`B` 0.03899 :`A` 1.0) (struct) 1.0 50.0)
      (bind _outactors (`GameplayStatics.GetAllActorsOfClass` "/Game/BP_Enemy/Guard_AI.Guard_AI_C"))
      (for _array_element _outactors
        (if (== (`/Game/BP_Enemy/Guard_AI.GroupID` _array_element) (`self.GroupID`))
          (`/Game/BP_Enemy/Guard_AI.Investigate` _array_element _returnvalue (`self.Patrol Points`))))
      (else
        (`KismetSystemLibrary.PrintString` "NotSeen")))
    (else
      (`KismetSystemLibrary.PrintString` "Lost Target")
      (`KismetSystemLibrary.DrawDebugBox` _returnvalue (0.0 0.0 0.0) (struct :`R` 0.798 :`B` 0.019875 :`A` 1.0) (struct) 1.0 50.0))))

(fn `UserConstructionScript`)